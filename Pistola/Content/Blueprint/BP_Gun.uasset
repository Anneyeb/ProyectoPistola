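; BP_Gun is a gun that fires BP_bala projectiles from a limited magazine and can be reloaded.
; The Disparar event spawns a bullet at the Arrow component's location and rotation while Municion remains, then decrements it and prints the remaining count, or prints an out-of-ammo message when empty.
; The Recargar event resets Municion to a full six-round magazine.
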(event Custom|Disparar
  (bind _arrow (Variables|Default|GetArrow))
  (bind _returnvalue (Transformation|GetWorldTransform _arrow))
  ;[0.15 0.15 0.15 0.5] Disparar: Crea la bala, si tiene balas resta las 6 balas del cargador y cuando no quedan te salta el mensjae "Sin balas".
  (if (> (Variables|Default|GetMunicion) 0)
    (Game|SpawnActorfromClass "/Game/Blueprint/BP_bala.BP_bala_C" (Math|Transform|MakeTransform (.location _returnvalue) (.rotation _returnvalue) "1.000000,1.000000,1.000000") "Undefined" "MultiplyWithRoot" 0 0)
    (Math|Integer|DecrementInt (Variables|Default|GetMunicion)
      (:%20%20
        (Development|PrintString (Utilities|String|ToString(Text) (Utilities|Text|FormatText "Te quedan {Municion} balas" (Variables|Default|GetMunicion))))))
    (else
      (Development|PrintString "Sin balas"))))

(event Custom|Recargar
  ;[0.15 0.15 0.15 0.5] Recarga 6 balas
  (Variables|Default|SetMunicion 6))

(fn ConstructionScript)