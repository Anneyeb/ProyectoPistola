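; BP_Enemigo is an enemy actor that appears as a random shape launched upward.
; On BeginPlay it sets the static mesh from RandomFiguras, randomizes its rotation and uniform scale, then applies a random upward velocity-change impulse.
; RandomFiguras selects among cone, tube and sphere meshes, but its random integer only yields the first two, so the sphere is never chosen.
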(event EventBeginPlay
  ;[0.15 0.15 0.15 0.5] Creacion del enemigo: En este evento se llama a la funcion random figuras, esta va al random transform que sirve para que las figuras tengan tamaños distintos y por ultimo toma un impulso para que las figuras vayan hacia arriba.
  (Components|StaticMesh|SetStaticMesh (Variables|Default|GetStaticMesh) (CallFunction|RandomFiguras))
  (Transformation|SetRelativeTransform (Variables|Default|GetStaticMesh) (Math|Transform|MakeTransform (Variables|/Script/Engine.SceneComponent|GetRelativeLocation (Variables|Default|GetStaticMesh)) (Math|Random|RandomRotator true) (Math|Conversions|ToVector(Float) (Math|Random|RandomFloatinRange 0.4 1.0))) false false)
  (Physics|AddImpulse (Variables|Default|GetStaticMesh) (Math|Vector|MakeVector 0.0 0.0 (Math|Random|RandomFloatinRange 7e+02 1.2e+03)) "None" true))

(fn ConstructionScript)

(fn RandomFiguras
  ;[0.15 0.15 0.15 0.5] RandomFiguras: Se crea la funcion para que aparezcan cualquiera de las 3 figuras de forma random y se especifica que haya un maximo de 2.
  (return (Utilities|Select :Index (Math|Random|RandomInteger 2) :Option%200 "/Game/StarterContent/Shapes/Shape_Cone.Shape_Cone" :Option%201 "/Game/StarterContent/Shapes/Shape_Tube.Shape_Tube" :Option%202 "/Game/StarterContent/Shapes/Shape_Sphere.Shape_Sphere")))