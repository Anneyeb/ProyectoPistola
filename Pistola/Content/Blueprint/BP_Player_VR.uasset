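; VR player Blueprint that picks up a pistol with the left controller and handles firing and reloading.
; Adds the pistol input mapping context on BeginPlay.
; The first gun overlapping the left controller mesh is destroyed, and a fresh BP_Gun spawns attached to the left motion controller while that mesh's visibility is turned off.
; An armed flag then lets the shoot and reload inputs forward to the held gun.
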(event OnComponentBeginOverlap(ControlMesh(Left))
  (params (OverlappedComponent :type Primitive%20Component%20Object%20Reference) (OtherActor :type Actor%20Object%20Reference) (OtherComp :type Primitive%20Component%20Object%20Reference) (OtherBodyIndex :type Integer) (bFromSweep :type Boolean) (SweepResult :type Hit%20Result%20Structure%20%28by%20ref%29))
  ;[0.15 0.15 0.15 0.5] Recoge el arma del suelo y la equipa en el personaje.
  (bind _asbp_gun (Utilities|Casting|CastToBP_Gun OtherActor))
  (Utilities|FlowControl|DoOnce false
    (:Completed
      (Actor|DestroyActor _asbp_gun)
      (Development|SetHiddeninGame (Variables|Default|GetControlMesh%28Left%29) false false)
      (bind _returnvalue (Game|SpawnActorfromClass "/Game/Blueprint/BP_Gun.BP_Gun_C" (Transformation|GetWorldTransform (Variables|Default|GetControlMesh%28Left%29)) "Undefined" "MultiplyWithRoot" 0 0))
      (bind _output_get (Variables|Default|SetGun _returnvalue))
      (Transformation|AttachComponentToComponent _output_get (Variables|Default|GetMotionController%20%28lefth%29) "None" "SnapToTarget" "SnapToTarget" "SnapToTarget" true)
      (Rendering|SetVisibility (Variables|Default|GetControlMesh%28Left%29) false false)
      (Variables|Default|SetArmado true))))

(event Input|EnhancedActionEvents|EnhancedInputActionIA_Disparar
  (params (ActionValue :type Boolean) (ElapsedSeconds :type Float%20%28double-precision%29) (TriggeredSeconds :type Float%20%28double-precision%29) (InputAction :type Input%20Action%20Object%20Reference :default "/Game/Input/IA_Disparar.IA_Disparar"))
  ;[0.15 0.15 0.15 0.5] Sistema de disparo.
  (:Started
    (if (Variables|Default|GetArmado)
      (Default|Disparar (Variables|Default|GetGun)))))

(event Input|EnhancedActionEvents|EnhancedInputActionIA_Recargar
  (params (ActionValue :type Boolean) (ElapsedSeconds :type Float%20%28double-precision%29) (TriggeredSeconds :type Float%20%28double-precision%29) (InputAction :type Input%20Action%20Object%20Reference :default "/Game/Input/IA_Recargar.IA_Recargar"))
  ;[0.15 0.15 0.15 0.5] Sistema de recarga
  (if (Variables|Default|GetArmado)
    (Default|Recargar (Variables|Default|GetGun))))

(event EventBeginPlay
  (Input|AddMappingContext (PlayerController|LocalPlayerSubsystems|GetEnhancedInputLocalPlayerSubsystem (Game|GetPlayerController 0)) "/Game/Input/IMC_Pistola.IMC_Pistola" 0 "(bIgnoreAllPressedKeysUntilRelease=True,bForceImmediately=False,bNotifyUserSettings=False)"))

(fn ConstructionScript)